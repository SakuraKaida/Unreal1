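; BP_Item is an item actor that vanishes with a sound when anything overlaps its Cylinder.
; BeginPlay spawns a tall, stretched ice-beam particle at its location as a glow, unattached and without auto-destroy.
; Overlap hides the Cylinder, sets a half-second lifespan and plays the sound at world origin, leaving collision enabled.
; The zero offset and BP_Item actor search at startup have no effect.
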(event `self.ReceiveBeginPlay`
  (`self.K2_AddActorLocalOffset` (`KismetMathLibrary.MakeVector` 0.0))
  (`GameplayStatics.GetAllActorsOfClass` "BP_Item_C")
  (if true
    (`GameplayStatics.SpawnEmitterAtLocation` "/Game/mae/InfinityBladeEffects/Effects/FX_Monsters/FX_Monster_Elemental/ICE/P_Beam_Impact_Ice.P_Beam_Impact_Ice" (`self.K2_GetActorLocation`) (struct) (0.3 0.3 20.0) false) ; 光るエフェクト
  ))

(event `self.Cylinder.OnComponentBeginOverlap`
  (params (OverlappedComponent :type "PrimitiveComponent Object Reference") (OtherActor :type "Actor Object Reference") (OtherComp :type "PrimitiveComponent Object Reference") (OtherBodyIndex :type Integer) (bFromSweep :type Boolean) (SweepResult :type "HitResult Structure (by ref)"))
  (`self.SetLifeSpan` 0.5) ; 消える時間
  (`SceneComponent.SetVisibility` (`self.Cylinder`) false false)
  (`GameplayStatics.PlaySoundAtLocation` "/Game/Sound/new/決定、ボタン押下47__online-audio-converter_com_.決定、ボタン押下47__online-audio-converter_com_" (0.0 0.0 0.0) (struct) 1.0 1.0 0.0 null null null) ; 音が鳴る
)

(fn `UserConstructionScript`)