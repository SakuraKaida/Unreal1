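; CAR_BP is a looping moving car hazard that deals very heavy damage to the player on contact.
; A timeline, with play rate set to the inverse of MainRate, lerps the mesh from StartPos to EndPos, then teleports it back and restarts.
; A box overlap with the player character applies the damage and plays a 2D explosion sound, gated to fire only once.
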(event `self.ReceiveBeginPlay`
  (bind _staticmesh (`self.StaticMesh`))
  (bind _startpos (`self.StartPos`))
  (`TimelineComponent.SetPlayRate` (`self.Control`) (/ 1.0 (`self.MainRate`)))
  (bind (_direction _rate) (`Timeline|Control` :!label _label)
    (:`Update`
      (`SceneComponent.K2_SetRelativeLocation` _staticmesh (`KismetMathLibrary.VLerp` _startpos (`self.EndPos`) _rate) false false))
    (:`Finished`
      (`SceneComponent.K2_SetRelativeLocation` _staticmesh _startpos false true)
      (goto _label :!via `PlayFromStart`))))

(event `self.Box.OnComponentBeginOverlap`
  (params (OverlappedComponent :type "PrimitiveComponent Object Reference") (OtherActor :type "Actor Object Reference") (OtherComp :type "PrimitiveComponent Object Reference") (OtherBodyIndex :type Integer) (bFromSweep :type Boolean) (SweepResult :type "HitResult Structure (by ref)"))
  (if (== OtherActor (`GameplayStatics.GetPlayerCharacter` 0))
    (`GameplayStatics.ApplyDamage` OtherActor 10000.0)
    (`/Engine/EditorBlueprintResources/StandardMacros.DoOnce` false
      (:`Completed`
        (`GameplayStatics.SpawnSound2D` "/Game/StarterContent/Audio/Explosion01.Explosion01" 2.0 1.0 0.0 null)))))

(fn `UserConstructionScript`)