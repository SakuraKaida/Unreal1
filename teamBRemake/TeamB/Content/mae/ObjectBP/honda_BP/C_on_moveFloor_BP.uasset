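; Moving floor actor that shuttles between two positions and carries a lethal trigger box.
; On BeginPlay a timeline, with play rate set from MainRate, lerps the StaticMesh's relative location from StartPos to EndPos.
; Each finish waits briefly, then flips the timeline's direction, so the motion repeats endlessly.
; When the player character begins overlapping the Box, it takes massive damage and an explosion sound plays.
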(event `self.ReceiveBeginPlay`
  (`TimelineComponent.SetPlayRate` (`self.Control`) (/ 1.0 (`self.MainRate`)))
  (bind (_direction _rate) (`Timeline|Control` :!label _label)
    (:`Update`
      (`SceneComponent.K2_SetRelativeLocation` (`self.StaticMesh`) (`KismetMathLibrary.VLerp` (`self.StartPos`) (`self.EndPos`) _rate) false false))
    (:`Finished`
      (`KismetSystemLibrary.Delay` 3.0)
      (switch `ETimelineDirection` _direction
        (:`Forward`
          (goto _label :!via `Reverse`))
        (:`Backward`
          (goto _label))))))

(event `self.Box.OnComponentBeginOverlap`
  (params (OverlappedComponent :type "PrimitiveComponent Object Reference") (OtherActor :type "Actor Object Reference") (OtherComp :type "PrimitiveComponent Object Reference") (OtherBodyIndex :type Integer) (bFromSweep :type Boolean) (SweepResult :type "HitResult Structure (by ref)"))
  (if (== OtherActor (`GameplayStatics.GetPlayerCharacter` 0))
    (`GameplayStatics.ApplyDamage` OtherActor 10000.0)
    (`GameplayStatics.SpawnSound2D` "/Game/StarterContent/Audio/Explosion01.Explosion01" 1.0 1.0 0.0 null)))

(fn `UserConstructionScript`)