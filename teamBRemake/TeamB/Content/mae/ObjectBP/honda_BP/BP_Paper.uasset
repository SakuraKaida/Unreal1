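; BP_Paper is a collectible paper item that awards points and increments the item count when the player overlaps it.
; Pickup spawns an effect and flip sound, destroys the actor, updates HUD_Score (cast from GameState), and prints a message once enough items are collected.
; A BeginPlay timeline moves it along local Z, spawning a tall heat-glow emitter with auto-destroy off on every update.
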(event `self.ReceiveActorBeginOverlap`
  (params (OtherActor :type "Actor Object Reference"))
  (if (== OtherActor (`GameplayStatics.GetPlayerCharacter` 0))
    (`GameplayStatics.SpawnEmitterAtLocation` "/Game/mae/InfinityBladeEffects/Effects/FX_Skill_Leap/P_Skill_Leap_Base_Charge_Weapon.P_Skill_Leap_Base_Charge_Weapon" (`self.K2_GetActorLocation`) (struct) (2.0 2.0 2.0))
    (`GameplayStatics.SpawnSound2D` "/Game/mae/ObjectBP/honda_BP/paper_sound/Book03-2_Flip__2.Book03-2_Flip__2" 2.0 1.0 0.0 null)
    (`self.K2_DestroyActor`)
    (bind _ashud_score (cast `/Game/mae/ThirdPersonBP/HUD_Score` (`GameplayStatics.GetGameState`)))
    (bind _output_get (set `/Game/mae/ThirdPersonBP/HUD_Score.ItemCount` (+ (`/Game/mae/ThirdPersonBP/HUD_Score.ItemCount` _ashud_score) 1) _ashud_score))
    (set `/Game/mae/ThirdPersonBP/HUD_Score.Score01` (+ (`/Game/mae/ThirdPersonBP/HUD_Score.Score01` _ashud_score) 2000) _ashud_score)
    (if (>= _output_get 5)
      (`KismetSystemLibrary.PrintString` "アイテムをすべて集めた"))))

(event `self.ReceiveBeginPlay`
  (bind (_direction `_新規track_0`) (`Timeline|タイムライン_0`)
    (:`Update`
      (`self.K2_AddActorLocalOffset` (`KismetMathLibrary.MakeVector` 0.0 0.0 `_新規track_0`))
      (`GameplayStatics.SpawnEmitterAtLocation` "/Game/mae/InfinityBladeEffects/Effects/FX_Cines/cinema03/P_CIN_IB_HeatGlow.P_CIN_IB_HeatGlow" (`self.K2_GetActorLocation`) (struct) (0.3 0.3 20.0) false))))

(fn `UserConstructionScript`)